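; Enemy AI controller that flies and fires a possessed BP_Spaceship relative to the player's pawn.
; A looping timer started on BeginPlay runs MoveAI, feeding normalized X and Y position offsets from the player into sideways and forward acceleration.
; When the ship is roughly aligned with the player on X, independent random rolls decide whether the left, middle and right missiles fire.
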(event `self.ReceiveBeginPlay`
  (`KismetSystemLibrary.K2_SetTimer` null "MoveAI" 0.2 true))

(event `self.ReceiveTick`
  (params (DeltaSeconds :type "Float (single-precision)")))

(fn `MoveAI`
  (bind _returnvalue (`KismetMathLibrary.RandomIntegerInRange` 1 3))
  (bind (_returnvalue_x _returnvalue_y) (`KismetMathLibrary.BreakVector` (`self.K2_GetActorLocation` (`self.K2_GetPawn` (`GameplayStatics.GetPlayerController` 0)))))
  (bind _asbp_spaceship (cast `/Game/Spaceship/Spaceship_BP/BP_Spaceship` (`self.K2_GetPawn`)))
  (`|ExecutionSequence`
    (:`then_0`
      (bind (_returnvalue_x_2 _returnvalue_y_2) (`KismetMathLibrary.BreakVector` (`self.K2_GetActorLocation` _asbp_spaceship)))
      (bind _returnvalue_2 (- _returnvalue_x_2 _returnvalue_x))
      (bind _returnvalue_3 (`KismetMathLibrary.NormalizeToRange` _returnvalue_2 -1.0 1.0))
      (`/Game/Spaceship/Spaceship_BP/BP_Spaceship.AccelerateSideways` _asbp_spaceship _returnvalue_3 _returnvalue_3))
    (:`then_1`
      (bind _returnvalue_4 (`KismetMathLibrary.NormalizeToRange` (- _returnvalue_y_2 _returnvalue_y) -1.0 1.0))
      (`/Game/Spaceship/Spaceship_BP/BP_Spaceship.AccelerateForward` _asbp_spaceship _returnvalue_4 _returnvalue_4))
    (:`then_2`
      (if (`KismetMathLibrary.InRange_FloatFloat` _returnvalue_2 -50.0 50.0)
        (`|ExecutionSequence`
          (:`then_0`
            (if (== _returnvalue 1)
              (`/Game/Spaceship/Spaceship_BP/BP_Spaceship.ShootLeftMissile` _asbp_spaceship)))
          (:`then_1`
            (if (== _returnvalue 2)
              (`/Game/Spaceship/Spaceship_BP/BP_Spaceship.ShootMiddleMissile` _asbp_spaceship)))
          (:`then_2`
            (if (== _returnvalue 3)
              (`/Game/Spaceship/Spaceship_BP/BP_Spaceship.ShootRightMissile` _asbp_spaceship))))))))

(fn `UserConstructionScript`)