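; Enemy spaceship Blueprint that flies and fires laser beams in response to input axes and actions, with no AI logic in its graphs.
; Forward and Left axes push the skeletal mesh with forces from arrow components, scaling only world Y for forward and X for sideways by the magnitude variables.
; Left and right missile actions spawn BP_LaserBeam at their shoot points; the middle action reuses the right point.
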(event `InputAxis|Forward`
  (params (AxisValue :type "Float (single-precision)"))
  (`self.AccelerateForward` AxisValue AxisValue))

(event `InputAction|LeftMissile`
  (params (Key :type "Key Structure"))
  (:`Pressed`
    (`|SpawnActorFromClass` "/Game/Spaceship/Weapons/BP_LaserBeam.BP_LaserBeam_C" (`SceneComponent.K2_GetComponentToWorld` (`self.ShootForwardLeft`)) "AlwaysSpawn" "OverrideRootScale" null null)))

(event `InputAxis|Left`
  (params (AxisValue :type "Float (single-precision)"))
  (`self.AccelerateSideways` AxisValue AxisValue))

(event `InputAction|RightMissile`
  (params (Key :type "Key Structure"))
  (:`Pressed`
    (`|SpawnActorFromClass` "/Game/Spaceship/Weapons/BP_LaserBeam.BP_LaserBeam_C" (`SceneComponent.K2_GetComponentToWorld` (`self.ShootForwardRight`)) "AlwaysSpawn" "OverrideRootScale" null null)))

(event `self.ReceiveTick`
  (params (DeltaSeconds :type "Float (single-precision)")))

(event `InputAction|MiddleMissile`
  (params (Key :type "Key Structure"))
  (:`Pressed`
    (`|SpawnActorFromClass` "/Game/Spaceship/Weapons/BP_LaserBeam.BP_LaserBeam_C" (`SceneComponent.K2_GetComponentToWorld` (`self.ShootForwardRight`)) "Undefined" "OverrideRootScale" null null)))

(fn `AccelerateForward`
  (params (A :type "Float (double-precision)") (A2 :type "Float (double-precision)"))
  (bind _skeletalmesh (`self.SkeletalMesh`))
  (bind _forwardarrow (`self.ForwardArrow`))
  (bind (_returnvalue_x _returnvalue_y _returnvalue_z) (`KismetMathLibrary.BreakVector` (`SceneComponent.GetForwardVector` _forwardarrow)))
  (bind (_returnvalue_x_2 _returnvalue_y_2 _returnvalue_z_2) (`KismetMathLibrary.BreakVector` (`SceneComponent.GetForwardVector` _forwardarrow)))
  (`|ExecutionSequence`
    (:`then_0`
      (if (>= A 0.1)
        (`PrimitiveComponent.AddForce` _skeletalmesh (`KismetMathLibrary.MakeVector` _returnvalue_x_2 (* _returnvalue_y_2 (`self.ForwardMagnitude`)) _returnvalue_z_2) "None" false)))
    (:`then_1`
      (if (<= A2 -0.1)
        (`PrimitiveComponent.AddForce` _skeletalmesh (`KismetMathLibrary.MakeVector` _returnvalue_x (* _returnvalue_y (* (`self.ForwardMagnitude`) -1.0)) _returnvalue_z) "None" false)))))

(fn `AccelerateSideways`
  (params (A :type "Float (double-precision)") (A2 :type "Float (double-precision)"))
  (bind _skeletalmesh (`self.SkeletalMesh`))
  (bind _sidearrow (`self.SideArrow`))
  (bind (_returnvalue_x _returnvalue_y _returnvalue_z) (`KismetMathLibrary.BreakVector` (`SceneComponent.GetForwardVector` _sidearrow)))
  (bind (_returnvalue_x_2 _returnvalue_y_2 _returnvalue_z_2) (`KismetMathLibrary.BreakVector` (`SceneComponent.GetForwardVector` _sidearrow)))
  (`|ExecutionSequence`
    (:`then_0`
      (if (>= A 0.1)
        (`PrimitiveComponent.AddForce` _skeletalmesh (`KismetMathLibrary.MakeVector` (* _returnvalue_x (`self.SideMagnitude`)) _returnvalue_y _returnvalue_z) "None" false)))
    (:`then_1`
      (if (<= A2 -0.1)
        (`PrimitiveComponent.AddForce` _skeletalmesh (`KismetMathLibrary.MakeVector` (* _returnvalue_x_2 (* (`self.SideMagnitude`) -1.0)) _returnvalue_y_2 _returnvalue_z_2) "None" false)))))

(fn `UserConstructionScript`)