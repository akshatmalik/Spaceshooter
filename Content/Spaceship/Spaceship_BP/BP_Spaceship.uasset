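; Player-controlled spaceship that flies by physics forces, fires laser beams and tracks its own health.
; Forward and sideways axis inputs push the skeletal mesh using arrow directions and snap it to fixed tilts.
; Three missile actions spawn BP_LaserBeam at muzzle components, with the middle shot reusing the right muzzle.
; ApplyDamage lowers Health, initialized in the construction script, but death is only checked on capsule overlap, which destroys the actor.
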(event `self.ReceiveTick`
  (params (DeltaSeconds :type "Float (single-precision)")))

(event `InputAxis|Forward`
  (params (AxisValue :type "Float (single-precision)"))
  (`self.AccelerateForward` AxisValue AxisValue))

(event `InputAction|LeftMissile`
  (params (Key :type "Key Structure"))
  (:`Pressed`
    (`self.ShootLeftMissile`)))

(event `self.ReceiveBeginPlay`)

(event `InputAction|RightMissile`
  (params (Key :type "Key Structure"))
  (:`Pressed`
    (`self.ShootRightMissile`)))

(event `InputAxis|Left`
  (params (AxisValue :type "Float (single-precision)"))
  (`self.AccelerateSideways` AxisValue AxisValue))

(event `InputAction|MiddleMissile`
  (params (Key :type "Key Structure"))
  (:`Pressed`
    (`self.ShootMiddleMissile`)))

(event `self.Capsule.OnComponentBeginOverlap`
  (params (OverlappedComponent :type "PrimitiveComponent Object Reference") (OtherActor :type "Actor Object Reference") (OtherComp :type "PrimitiveComponent Object Reference") (OtherBodyIndex :type Integer) (bFromSweep :type Boolean) (SweepResult :type "HitResult Structure (by ref)"))
  (`self.CheckHealth`))

(fn `AccelerateForward`
  (params (A :type "Float (double-precision)") (A2 :type "Float (double-precision)"))
  (bind _returnvalue (>= A 0.1))
  (bind _returnvalue_2 (<= A2 -0.1))
  (bind _skeletalmesh (`self.SkeletalMesh`))
  (bind _forwardarrow (`self.ForwardArrow`))
  (bind (_returnvalue_x _returnvalue_y _returnvalue_z) (`KismetMathLibrary.BreakVector` (`SceneComponent.GetForwardVector` _forwardarrow)))
  (bind (_returnvalue_x_2 _returnvalue_y_2 _returnvalue_z_2) (`KismetMathLibrary.BreakVector` (`SceneComponent.GetForwardVector` _forwardarrow)))
  (`|ExecutionSequence`
    (:`then_0`
      (set `self.IsMovingForward` _returnvalue)
      (if _returnvalue
        (`PrimitiveComponent.AddForce` _skeletalmesh (`KismetMathLibrary.MakeVector` _returnvalue_x_2 (* _returnvalue_y_2 (`self.ForwardMagnitude`)) _returnvalue_z_2) "None" false)
        (`SceneComponent.K2_SetRelativeRotation` (`self.SkeletalMesh`) (struct :`Roll` -80.0) true true)))
    (:`then_1`
      (set `self.IsMovingBackward` _returnvalue_2)
      (if _returnvalue_2
        (`PrimitiveComponent.AddForce` _skeletalmesh (`KismetMathLibrary.MakeVector` _returnvalue_x (* _returnvalue_y (* (`self.ForwardMagnitude`) -1.0)) _returnvalue_z) "None" false)
        (`SceneComponent.K2_SetRelativeRotation` (`self.SkeletalMesh`) (struct :`Roll` 80.0) true true)))))

(fn `AccelerateSideways`
  (params (A :type "Float (double-precision)") (A2 :type "Float (double-precision)"))
  (bind _returnvalue (>= A 0.1))
  (bind _returnvalue_2 (<= A2 -0.1))
  (bind _skeletalmesh (`self.SkeletalMesh`))
  (bind _sidearrow (`self.SideArrow`))
  (bind (_returnvalue_x _returnvalue_y _returnvalue_z) (`KismetMathLibrary.BreakVector` (`SceneComponent.GetForwardVector` _sidearrow)))
  (bind (_returnvalue_x_2 _returnvalue_y_2 _returnvalue_z_2) (`KismetMathLibrary.BreakVector` (`SceneComponent.GetForwardVector` _sidearrow)))
  (`|ExecutionSequence`
    (:`then_0`
      (set `self.IsMovingLeft` _returnvalue)
      (if _returnvalue
        (`PrimitiveComponent.AddForce` _skeletalmesh (`KismetMathLibrary.MakeVector` (* _returnvalue_x (`self.SideMagnitude`)) _returnvalue_y _returnvalue_z) "None" false)
        (`SceneComponent.K2_SetRelativeRotation` (`self.SkeletalMesh`) (struct :`Pitch` 80.0) true true)))
    (:`then_1`
      (set `self.IsMovingRight` _returnvalue_2)
      (if _returnvalue_2
        (`PrimitiveComponent.AddForce` _skeletalmesh (`KismetMathLibrary.MakeVector` (* _returnvalue_x_2 (* (`self.SideMagnitude`) -1.0)) _returnvalue_y_2 _returnvalue_z_2) "None" false)
        (`SceneComponent.K2_SetRelativeRotation` (`self.SkeletalMesh`) (struct :`Pitch` -80.0) true true)))))

(fn `ApplyDamage`
  (params (Damage :type "Float (double-precision)"))
  (set `self.Health` (- (`self.Health`) Damage)))

(fn `CheckHealth`
  (if (<= (`self.Health`) 0.0)
    (`KismetSystemLibrary.PrintString` "Dead")
    (`self.K2_DestroyActor`)))

(fn `ShootLeftMissile`
  (bind (_returnvalue_location _returnvalue_rotation) (`KismetMathLibrary.BreakTransform` (`SceneComponent.K2_GetComponentToWorld` (`self.ShootForwardLeft`))))
  (`|SpawnActorFromClass` "/Game/Spaceship/Weapons/BP_LaserBeam.BP_LaserBeam_C" (`KismetMathLibrary.MakeTransform` _returnvalue_location _returnvalue_rotation (0.2 0.2 0.2)) "AlwaysSpawn" "OverrideRootScale" null null))

(fn `ShootMiddleMissile`
  (bind (_returnvalue_location _returnvalue_rotation) (`KismetMathLibrary.BreakTransform` (`SceneComponent.K2_GetComponentToWorld` (`self.ShootForwardRight`))))
  (`|SpawnActorFromClass` "/Game/Spaceship/Weapons/BP_LaserBeam.BP_LaserBeam_C" (`KismetMathLibrary.MakeTransform` _returnvalue_location _returnvalue_rotation (0.2 0.2 0.2)) "Undefined" "OverrideRootScale" null null))

(fn `ShootRightMissile`
  (bind (_returnvalue_location _returnvalue_rotation) (`KismetMathLibrary.BreakTransform` (`SceneComponent.K2_GetComponentToWorld` (`self.ShootForwardRight`))))
  (`|SpawnActorFromClass` "/Game/Spaceship/Weapons/BP_LaserBeam.BP_LaserBeam_C" (`KismetMathLibrary.MakeTransform` _returnvalue_location _returnvalue_rotation (0.2 0.2 0.2)) "AlwaysSpawn" "OverrideRootScale" null null))

(fn `UserConstructionScript`
  (set `self.Health` (`self.MaxHealth`)))